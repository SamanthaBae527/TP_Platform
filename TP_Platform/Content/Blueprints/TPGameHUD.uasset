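; HUD Blueprint that both holds the game state and draws it for a timed coin-collecting game.
; StartGame resets score, flags and countdown on BeginPlay, then a looping one-second timer decrements Time until game over.
; CoinCollected raises Score and grants HasKey at ten coins, while ClockCollected adds time.
; DrawHUD draws time and score, plus game-over text with final score and a win message if HasKey is set.
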(event `timer`
  ;[1 1 1] timer
  (bind _result (`/Engine/EditorBlueprintResources/StandardMacros.DecrementInt` (`self.time`))
    (:`  `
      (if (<= _result 0)
        (set `self.gameOver` true)
        (`KismetSystemLibrary.K2_ClearTimer` null "timer")))))

(event `self.ReceiveBeginPlay`
  (`self.StartGame`))

(event `self.ReceiveDrawHUD`
  (params (SizeX :type Integer) (SizeY :type Integer))
  ;[1 1 1] Score/Time/GameOver/Win/Loss Text Drawing
  (`self.DrawText` (`KismetStringLibrary.Conv_IntToString` (`self.time`)) (struct :`A` 1) 0.0 0.0 null 3.0)
  (`self.DrawText` (`KismetStringLibrary.Conv_IntToString` (`self.score`)) (struct :`A` 1) 500.0 10.0 null 3.0)
  (if (`self.gameOver`)
    (`self.DrawText` "GAME OVER" (struct :`R` 0.019444 :`G` 0.327911 :`B` 0.466667 :`A` 1.0) 200.0 200.0 null 5.0)
    (`self.DrawText` "Final Score:" (struct :`R` 0.716667 :`B` 0.56913 :`A` 1.0) 500.0 500.0 null 2.0)
    (`self.DrawText` (`KismetStringLibrary.Conv_IntToString` (`self.score`)) (struct :`R` 1.0 :`B` 0.777425 :`A` 1.0) 650.0 500.0 null 2.0)
    (if (`self.hasKey`)
      (`self.DrawText` "YOU WIN" (struct :`R` 0.904167 :`G` 0.372969 :`B` 0.529616 :`A` 1.0) 700.0 300.0 null 5.0))))

(fn `ClockCollected`
  (set `self.time` (+ (`self.time`) 5)))

(fn `CoinCollected`
  (bind _result (`/Engine/EditorBlueprintResources/StandardMacros.IncrementInt` (`self.score`))
    (:`  `
      (if (== (`KismetMathLibrary.Conv_IntToInt64` _result) 10)
        (set `self.hasKey` true)))))

(fn `UserConstructionScript`)